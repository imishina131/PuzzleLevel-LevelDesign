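; BP_RoomTrigger is a trigger box that randomly picks one of three pre-placed room variants when first overlapped by anything.
; It hides the Room01, Room02 and Room03 actor arrays, then unhides one at random.
; After a one-second delay, it disables collision on the other two and only then sets HasSpawned to block repeats.
; An unconnected older branch instead streams a random room level at EndPivot for the first-person character.
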(event `self.Box.OnComponentBeginOverlap`
  (params (OverlappedComponent :type "PrimitiveComponent Object Reference") (OtherActor :type "Actor Object Reference") (OtherComp :type "PrimitiveComponent Object Reference") (OtherBodyIndex :type Integer) (bFromSweep :type Boolean) (SweepResult :type "HitResult Structure (by ref)"))
  (if (not (`self.HasSpawned`))
    (for _array_element (`self.Room03`)
      (`self.SetActorHiddenInGame` _array_element true))
    (for _array_element_2 (`self.Room02`)
      (`self.SetActorHiddenInGame` _array_element_2 true))
    (for _array_element_3 (`self.Room01`)
      (`self.SetActorHiddenInGame` _array_element_3 true))
    (switch `int` (`KismetMathLibrary.RandomIntegerInRange` 0 2)
      (:`0`
        (for _array_element_4 (`self.Room01`)
          (`self.SetActorHiddenInGame` _array_element_4 false)
          (`KismetSystemLibrary.Delay` 1.0)
          (`self.SetActorEnableCollision` (`self.Room02`) false)
          (`self.SetActorEnableCollision` (`self.Room03`) false)
          (set `self.HasSpawned` true)))
      (:`1`
        (for _array_element_5 (`self.Room02`)
          (`self.SetActorHiddenInGame` _array_element_5 false)
          (`KismetSystemLibrary.Delay` 1.0)
          (`self.SetActorEnableCollision` (`self.Room01`) false)
          (`self.SetActorEnableCollision` (`self.Room03`) false)
          (set `self.HasSpawned` true)))
      (:`2`
        (for _array_element_6 (`self.Room03`)
          (`self.SetActorHiddenInGame` _array_element_6 false)
          (`KismetSystemLibrary.Delay` 1.0)
          (`self.SetActorEnableCollision` (`self.Room01`) false)
          (`self.SetActorEnableCollision` (`self.Room02`) false)
          (set `self.HasSpawned` true))))))

(fn `UserConstructionScript`)